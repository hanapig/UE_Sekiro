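; AI enemy character Blueprint providing a library of melee, ranged, evasion and reaction moves against the player.
; It caches the MySCharacter player on BeginPlay and updates that player's location every Tick.
; Each move function plays a montage, with many first setting a named Motion Warping target at the player's location.
; Some attacks also update AttackTags, while the parry stagger (弹反僵直) swaps the player's BlockTags from Stiff to Hurt.
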(event `self.ReceiveBeginPlay`
  (bind _returnvalue (`GameplayStatics.GetActorOfClass` "/Game/Character/MySCharacter.MySCharacter_C"))
  (set `self.Player1` _returnvalue))

(event `self.ReceiveTick`
  (params (DeltaSeconds :type "Float (single-precision)"))
  (set `self.PlayerLoction` (`self.K2_GetActorLocation` (`self.Player1`))))

(fn `Over`)

(fn `Start_Att1`
  (`BlueprintGameplayTagLibrary.AddGameplayTag` (`self.AttackTags`) (struct :`TagName` "Rolling"))
  (`MotionWarpingComponent.AddOrUpdateWarpTarget` (`self.MotionWarping`) (make `MotionWarpingTarget` "point1" (`self.K2_GetActorLocation` (`self.Player1`))))
  (`self.PlayAnimMontage` "/Game/AI_Anim/AI_Montage_Att1.AI_Montage_Att1"))

(fn `StartCombo_Spike`
  (`MotionWarpingComponent.AddOrUpdateWarpTarget` (`self.MotionWarping`) (make `MotionWarpingTarget` "point12" (`self.PlayerLoction`)))
  (`self.PlayAnimMontage` "/Game/AI_Anim/att2_ai_Montage.att2_ai_Montage"))

(fn `test1`
  (`BlueprintGameplayTagLibrary.RemoveGameplayTag` (`self.AttackTags`) (struct :`TagName` "Rolling"))
  (`MotionWarpingComponent.AddOrUpdateWarpTarget` (`self.MotionWarping`) (make `MotionWarpingTarget` "point2" (`self.K2_GetActorLocation` (`self.Player1`))))
  (`self.PlayAnimMontage` "/Game/AI_Anim/AI_Attack1.AI_Attack1"))

(fn `test2`
  (`MotionWarpingComponent.AddOrUpdateWarpTarget` (`self.MotionWarping`) (make `MotionWarpingTarget` "point2" (`self.K2_GetActorLocation` (`self.Player1`))))
  (`self.PlayAnimMontage` "/Game/AI_Anim/AI_Attack2.AI_Attack2"))

(fn `UserConstructionScript`)

(fn `侧身连斩`
  (`BlueprintGameplayTagLibrary.AddGameplayTag` (`self.AttackTags`) (struct :`TagName` "Combo"))
  (`MotionWarpingComponent.AddOrUpdateWarpTarget` (`self.MotionWarping`) (make `MotionWarpingTarget` "point7" (`self.PlayerLoction`)))
  (`self.PlayAnimMontage` "/Game/AI_Anim/侧身跑连续斩_Montage.侧身跑连续斩_Montage"))

(fn `单发`
  (`self.PlayAnimMontage` "/Game/AI_Anim/one.one"))

(fn `受击`
  (`self.PlayAnimMontage` "/Game/AI_Anim/AI_Montage_Att1.AI_Montage_Att1"))

(fn `右撤追击`
  (`MotionWarpingComponent.AddOrUpdateWarpTarget` (`self.MotionWarping`) (make `MotionWarpingTarget` "point15" (`self.PlayerLoction`)))
  (`self.PlayAnimMontage` "/Game/AI_Anim/Left_Combo.Left_Combo"))

(fn `右跑`
  (`self.PlayAnimMontage` "/Game/AI_Anim/Left_Run_Montage.Left_Run_Montage"))

(fn `后撤`
  (`self.PlayAnimMontage` "/Game/AI_Anim/快速后撤_Montage.快速后撤_Montage")
  (`KismetSystemLibrary.K2_SetTimerDelegate` :`Time` 2.0))

(fn `射箭`
  (`MotionWarpingComponent.AddOrUpdateWarpTarget` (`self.MotionWarping`) (make `MotionWarpingTarget` "point10" (`self.K2_GetActorLocation` (`self.Player1`))))
  (`self.PlayAnimMontage` "/Game/AI_Anim/two_Montage.two_Montage"))

(fn `弹反僵直`
  (`self.PlayAnimMontage` "/Game/AI_Anim/弹反僵直_Montage.弹反僵直_Montage")
  (bind _asscharacter (cast `SCharacter` (`self.Player1`)))
  (bind _blocktags (`SCharacter.BlockTags` _asscharacter))
  (`BlueprintGameplayTagLibrary.RemoveGameplayTag` _blocktags (struct :`TagName` "Stiff"))
  (`BlueprintGameplayTagLibrary.AddGameplayTag` _blocktags (struct :`TagName` "Hurt")))

(fn `普通攻击`
  (`MotionWarpingComponent.AddOrUpdateWarpTarget` (`self.MotionWarping`) (make `MotionWarpingTarget` "point2" (`self.PlayerLoction`)))
  (`self.PlayAnimMontage` "/Game/AI_Anim/AI_Attack2.AI_Attack2"))

(fn `横斩`
  (bind _attacktags (`self.AttackTags`))
  (`BlueprintGameplayTagLibrary.RemoveGameplayTag` _attacktags (struct :`TagName` "Rolling"))
  (`BlueprintGameplayTagLibrary.AddGameplayTag` _attacktags (struct :`TagName` "Combo3"))
  (`MotionWarpingComponent.AddOrUpdateWarpTarget` (`self.MotionWarping`) (make `MotionWarpingTarget` "point14" (`self.PlayerLoction`)))
  (`self.PlayAnimMontage` "/Game/AI_Anim/横斩_Montage.横斩_Montage"))

(fn `突刺`
  (`BlueprintGameplayTagLibrary.AddGameplayTag` (`self.AttackTags`) (struct :`TagName` "Spikes"))
  (`MotionWarpingComponent.AddOrUpdateWarpTarget` (`self.MotionWarping`) (make `MotionWarpingTarget` "point4" (`self.K2_GetActorLocation` (`self.Player1`))))
  (`self.PlayAnimMontage` "/Game/AI_Anim/突刺.突刺"))

(fn `跳劈`
  (`BlueprintGameplayTagLibrary.AddGameplayTag` (`self.AttackTags`) (struct :`TagName` "LeapAttack"))
  (`MotionWarpingComponent.AddOrUpdateWarpTarget` (`self.MotionWarping`) (make `MotionWarpingTarget` "point3" (`self.K2_GetActorLocation` (`self.Player1`))))
  (`self.PlayAnimMontage` "/Game/AI_Anim/重劈_Montage.重劈_Montage"))

(fn `踢击`
  (`self.PlayAnimMontage` "/Game/AI_Anim/Foot_Combo_Montage.Foot_Combo_Montage"))

(fn `追击`
  (`BlueprintGameplayTagLibrary.AddGameplayTag` (`self.AttackTags`) (struct :`TagName` "Rolling"))
  (`MotionWarpingComponent.AddOrUpdateWarpTarget` (`self.MotionWarping`) (make `MotionWarpingTarget` "point11" (`self.PlayerLoction`)))
  (`self.PlayAnimMontage` "/Game/AI_Anim/FollowAttack_Montage.FollowAttack_Montage"))